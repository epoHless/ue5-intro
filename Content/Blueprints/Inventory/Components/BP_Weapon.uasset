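; Weapon inventory component that holds projectile types in slots and fires the selected one from an object pool.
; BeginPlay builds the slots and pre-spawns disabled pool objects; shooting moves a free one into position and passes it the current slot's data and direction.
; An exhausted pool spawns another object but returns none for that request.
; Slot changes and projectiles added to the first empty slot are broadcast through events.
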(event `self.ReceiveBeginPlay`
  (`self.Init Weapon`)
  (`self.Init Pool` (`self.Pool Size`)))

(event `On Shoot`
  (params (Forward :type "Vector Structure") (Position :type "Vector Structure"))
  (bind _object (`self.Get Object`))
  (`Actor.K2_SetActorLocation` _object Position false false)
  (`/Game/Blueprints/Inventory/Projectiles/BP_Projectile.On Object Request` _object (`/Game/Blueprints/Inventory/Components/InventorySlot.CurrentItem` (`self.Current Slot`)) Forward))

(fn `Add Projectile`
  (params (Data :type "/Game/Blueprints/Inventory/Projectiles/DA_Projectile Object Reference"))
  (for (_array_element _array_index) (`self.Slots`)
    (`/Engine/EditorBlueprintResources/StandardMacros.IsValid` (`/Game/Blueprints/Inventory/Components/InventorySlot.CurrentItem` _array_element)
      (:`Is Not Valid`
        (bind _output_get (set `/Game/Blueprints/Inventory/Components/InventorySlot.CurrentItem` Data _array_element))
        (`self.OnBulletAdded` _output_get _array_index)
        (return)))))

(fn `Get Object`
  (returns (Object :type "/Game/Blueprints/Inventory/Projectiles/BP_Projectile Object Reference"))
  (for _array_element (`self.Spawned Objects`)
    (if (not (`/Game/Blueprints/Inventory/Projectiles/BP_Projectile.bEnabled` _array_element))
      (return _array_element)))
  (`self.Init Pool` 1))

(fn `Init Pool`
  (params (Size :type Integer))
  (for _ (range Size)
    (bind _returnvalue (`|SpawnActorFromClass` (`self.ObjectToPool`) (`KismetMathLibrary.MakeTransform` (0.0 0.0 0.0)) "Undefined" "MultiplyWithRoot" null null))
    (`KismetArrayLibrary.Array_Add` (`self.Spawned Objects`) _returnvalue)
    (`/Game/Blueprints/Inventory/Projectiles/BP_Projectile.Toggle Object` _returnvalue false)))

(fn `Init Weapon`
  (for _ (range (`self.Size`))
    (bind _returnvalue (`|GenericCreateObject` "/Game/Blueprints/Inventory/Components/InventorySlot.InventorySlot_C"))
    (`KismetArrayLibrary.Array_Add` (`self.Slots`) _returnvalue))
  (set `self.Current Slot` (`|GetArrayItem` (`self.Slots`))))

(fn `Set Slot`
  (params (Direction :type Integer))
  (returns (Slot :type "/Game/Blueprints/Inventory/Components/InventorySlot Object Reference"))
  (locals (`Target Index` :type Integer))
  (bind _output_get (set `local.Target Index` (+ (`KismetArrayLibrary.Array_Find` (`self.Slots`) (`self.Current Slot`)) Direction)))
  (if (>= _output_get (- (`KismetArrayLibrary.Array_Length` (`self.Slots`)) 1))
    (set `local.Target Index` 0))
  (if (< (`local.Target Index`) 0)
    (set `local.Target Index` (- (`KismetArrayLibrary.Array_Length` (`self.Slots`)) 1)))
  (bind _output_get_2 (set `self.Current Slot` (`|GetArrayItem` (`self.Slots`) (`local.Target Index`))))
  (`self.OnSlotChanged` _output_get_2)
  (return _output_get_2))