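; BP_Projectile is a reusable projectile, activated and deactivated through object request and release events, as in object pooling.
; A request orients it along a direction, switches on collision, tick and visibility, and sets velocity from the supplied data's speed.
; A sphere overlap applies the data's damage to the other actor, then releases the projectile by hiding and disabling it instead of destroying it.
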(event `On Object Request`
  (params (Data :type "/Game/Blueprints/Inventory/Projectiles/DA_Projectile Object Reference") (Direction :type "Vector Structure"))
  (`self.K2_SetActorRotation` (`KismetMathLibrary.Conv_VectorToRotator` Direction))
  (`self.Toggle Object` true)
  (`self.Set Data` Data)
  (set `self.bEnabled` true))

(event `On Object Release`
  (`self.Toggle Object` false)
  (set `self.bEnabled` false))

(event `self.Sphere.OnComponentBeginOverlap`
  (params (OverlappedComponent :type "PrimitiveComponent Object Reference") (OtherActor :type "Actor Object Reference") (OtherComp :type "PrimitiveComponent Object Reference") (OtherBodyIndex :type Integer) (bFromSweep :type Boolean) (SweepResult :type "HitResult Structure (by ref)"))
  (`GameplayStatics.ApplyDamage` OtherActor (`/Game/Blueprints/Inventory/Projectiles/DA_Projectile.Damage` (`self.CurrentData`)))
  (`self.On Object Release`))

(fn `Set Data`
  (params (Data :type "/Game/Blueprints/Inventory/Projectiles/DA_Projectile Object Reference"))
  (bind _output_get (set `self.CurrentData` Data))
  (set `MovementComponent.Velocity` (* (`/Game/Blueprints/Inventory/Projectiles/DA_Projectile.Speed` _output_get) (`self.GetActorForwardVector`)) (`self.ProjectileMovement`)))

(fn `Toggle Object`
  (params (Toggle :type Boolean))
  (locals (Collision :type "ECollisionEnabled Enum"))
  (if Toggle
    (set `local.Collision` "QueryAndPhysics")
    (else
      (set `local.Collision` "NoCollision")))
  (`PrimitiveComponent.SetCollisionEnabled` (`self.Sphere`) (`local.Collision`))
  (`self.SetActorTickEnabled` Toggle)
  (`self.SetActorHiddenInGame` (not Toggle)))

(fn `UserConstructionScript`)