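; GM_Standard, apparently the standard game mode, sets up the inventory UI and links it to the player's inventory.
; On BeginPlay it creates WB_Inventory, adds it to the viewport, and initializes its slots from the BP_Player InventoryComponent's size.
; It binds to that component's events, forwarding added bullets to the widget by slot index.
; The slot-changed handler is bound but empty.
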(event `self.ReceiveBeginPlay`
  (bind _returnvalue (`|CreateWidget` "/Game/Blueprints/Inventory/UI/WB_Inventory.WB_Inventory_C"))
  (bind _output_get (set `self.Inventory UI` _returnvalue))
  (`UserWidget.AddToViewport` _output_get 0)
  (bind _asbp_player (cast `/Game/Blueprints/BP_Player` (`GameplayStatics.GetPlayerCharacter` 0)))
  (bind _output_get_2 (set `self.Player` _asbp_player))
  (bind _inventory_component (`/Game/Blueprints/BP_Player.Inventory Component` _output_get_2))
  (`/Game/Blueprints/Inventory/UI/WB_Inventory.Init Slots` (`self.Inventory UI`) (`/Game/Blueprints/Inventory/Components/BP_Weapon.Size` _inventory_component))
  (add `/Game/Blueprints/Inventory/Components/BP_Weapon.OnBulletAdded` _inventory_component (delegate `OnBulletAdded_Event`))
  (add `/Game/Blueprints/Inventory/Components/BP_Weapon.OnSlotChanged` _inventory_component (delegate `OnSlotChanged_Event`)))

(event `OnSlotChanged_Event`
  (params (Slot :type "/Game/Blueprints/Inventory/Components/InventorySlot Object Reference")))

(event `OnBulletAdded_Event`
  (params (Data :type "/Game/Blueprints/Inventory/Projectiles/DA_Projectile Object Reference") (Index :type Integer))
  (`/Game/Blueprints/Inventory/UI/WB_Inventory.AddBulletToSlot` (`self.Inventory UI`) Data Index))

(fn `UserConstructionScript`)