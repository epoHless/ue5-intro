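; BP_Player is the player actor, mapping input to movement, yaw rotation, inventory slot switching and shooting.
; An InventoryComponent handles slot changes, which print the current item, and receives Arrow1's forward vector and location for shooting.
; The Horizontal axis moves along a world-space X/Y diagonal, while Vertical is unimplemented.
; AnyDamage sets Health to Damage minus Health, reversing the usual subtraction, and destroys the actor at zero or below.
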(event `InputAction|InventoryUp`
  (params (Key :type "Key Structure"))
  (:`Pressed`
    (bind _slot (`/Game/Blueprints/Inventory/Components/BP_Weapon.Set Slot` (`self.Inventory Component`) 1))
    (`KismetSystemLibrary.PrintString` (`KismetStringLibrary.Concat_StrStr` "New Slot : " (`KismetSystemLibrary.GetDisplayName` (`/Game/Blueprints/Inventory/Components/InventorySlot.CurrentItem` _slot))) :!label _label)))

(event `InputAxis|Horizontal`
  (params (AxisValue :type "Float (single-precision)"))
  (`self.AddMovementInput` (`KismetMathLibrary.MakeVector` (stale `InputAxis|Vertical` AxisValue) AxisValue)))

(event `InputAxis|Vertical`
  (params (AxisValue :type "Float (single-precision)")))

(event `InputAction|InventoryDown`
  (params (Key :type "Key Structure"))
  (:`Pressed`
    (`/Game/Blueprints/Inventory/Components/BP_Weapon.Set Slot` (`self.Inventory Component`) -1)
    (goto _label)))

(event `InputAxis|Rotation`
  (params (AxisValue :type "Float (single-precision)"))
  (`self.AddControllerYawInput` AxisValue))

(event `InputAction|Shoot`
  (params (Key :type "Key Structure"))
  (bind _arrow1 (`self.Arrow1`))
  (:`Pressed`
    (`/Game/Blueprints/Inventory/Components/BP_Weapon.On Shoot` (`self.Inventory Component`) (`SceneComponent.GetForwardVector` _arrow1) (`SceneComponent.K2_GetComponentLocation` _arrow1))))

(event `self.ReceiveAnyDamage`
  (params (Damage :type "Float (single-precision)") (DamageType :type "DamageType Object Reference") (InstigatedBy :type "Controller Object Reference") (DamageCauser :type "Actor Object Reference"))
  (bind _output_get (set `self.Health` (- Damage (`self.Health`))))
  (if (<= _output_get 0.0)
    (`self.K2_DestroyActor`)))

(fn `UserConstructionScript`)